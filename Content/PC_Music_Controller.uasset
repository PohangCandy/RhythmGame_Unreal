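; Player controller for a music game that forwards Space presses to the GM_Music game mode.
; On BeginPlay it casts and caches the game mode as GM_Music.
; On a Space press it checks the game mode's YPos and, if it is above a fixed threshold, prints a debug string and triggers CallGMCollision on the game mode.
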(event `self.ReceiveBeginPlay`
  (bind _asgm_music (cast `/Game/GM_Music` (`GameplayStatics.GetGameMode`)))
  (set `self.As GM Music` _asgm_music))

(event `InputAction|Space_Pressed`
  (params (Key :type "Key Structure"))
  (:`Pressed`
    (if (> (`/Game/GM_Music.Y_Pos` (`self.As GM Music`)) 500.0)
      (`KismetSystemLibrary.PrintString` "Hi collision" true true (struct :`R` 1.0 :`B` 0.088987 :`A` 1.0) 5.0)
      (`/Game/GM_Music.GM_Collision` (`self.As GM Music`)))))

(fn `UserConstructionScript`)